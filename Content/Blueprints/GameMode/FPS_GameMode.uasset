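; Game mode for a timed FPS round where the player must clear the zone of drones.
; Tick drives a session state enum from warm-up countdown into the game timer, ending in out of time.
; It creates the HUD and updates timers, drone count and announcements, with functions for drone death, win and loss.
; The win check and input-disabling logic are disconnected, so neither runs.
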(event `self.ReceiveBeginPlay`
  (bind _hud (`self.HUD`))
  (`|ExecutionSequence`
    (:`then_0`
      ; Set HUD
      (bind _returnvalue (`|GenericCreateObject` "/Game/Blueprints/HUD/GameModeHUD.GameModeHUD_C"))
      (bind _output_get (set `self.HUD` _returnvalue))
      (`UserWidget.AddToViewport` _output_get 0)
      (set `TextBlock.Text` "Clear the ZONE!" (`/Game/Blueprints/HUD/GameModeHUD.Announcement` _hud))
      (bind _formattime (`self.ToTimeFormat` (`self.GameTime`)))
      (set `TextBlock.Text` _formattime (`/Game/Blueprints/HUD/GameModeHUD.TimeText` _hud)))
    (:`then_1`
      ; Set Drone Text
      (bind _outactors (`GameplayStatics.GetAllActorsOfClass` "/Game/Blueprints/Drone/Drone.Drone_C"))
      (bind _output_get_2 (set `self.DroneNum` (`KismetArrayLibrary.Array_Length` _outactors)))
      (set `TextBlock.Text` (`KismetTextLibrary.Conv_IntToText` _output_get_2) (`/Game/Blueprints/HUD/GameModeHUD.DroneText` (`self.HUD`))))
    (:`then_2`
      (`self.DisablePlayerInput`))))

(event `self.ReceiveTick`
  (params (DeltaSeconds :type "Float (single-precision)"))
  (bind _announcement (`/Game/Blueprints/HUD/GameModeHUD.Announcement` (`self.HUD`)))
  (switch `/Game/Blueprints/GameMode/SessionStates` (`self.SessionStates`)
    (:`NewEnumerator0`
      (bind _finished (`self.UpdateWarmup`))
      (if _finished
        (set `self.SessionStates` "NewEnumerator1")
        (`self.StartGame`)))
    (:`NewEnumerator1`
      (bind _finished_2 (`self.UpdateGameTimer` DeltaSeconds))
      (if _finished_2
        (set `self.SessionStates` "NewEnumerator2")
        (`self.DisablePlayerInput`)
        (`Widget.SetIsEnabled` _announcement true)
        (set `TextBlock.Text` "YOU are OUT OF TIME!" _announcement)))))

(fn `DisablePlayerInput`)

(fn `DroneDied`
  (bind _result (`/Engine/EditorBlueprintResources/StandardMacros.DecrementInt` (`self.DroneNum`))
    (:`  `
      (bind _output_get (set `self.DroneNum` _result))
      (set `TextBlock.Text` (`KismetTextLibrary.Conv_IntToText` _output_get) (`/Game/Blueprints/HUD/GameModeHUD.DroneText` (`self.HUD`)))
      ; Check winning conditions
      (if (<= (`self.DroneNum`) 0)
        _))))

(fn `PlayerDied`
  (bind _hud (`self.HUD`))
  (bind _announcement (`/Game/Blueprints/HUD/GameModeHUD.Announcement` _hud))
  (set `self.SessionStates` "NewEnumerator3")
  (`Widget.SetIsEnabled` _announcement true)
  (set `TextBlock.Text` " GAME OVER, L!" _announcement)
  (set `TextBlock.Text` "00:00" (`/Game/Blueprints/HUD/GameModeHUD.TimeText` _hud))
  (`self.DisablePlayerInput`))

(fn `PlayerWon`
  (bind _announcement (`/Game/Blueprints/HUD/GameModeHUD.Announcement` (`self.HUD`)))
  (set `self.SessionStates` "NewEnumerator4")
  (`Widget.SetIsEnabled` _announcement true)
  (set `TextBlock.Text` "You've WONNNN" _announcement)
  (`self.DisablePlayerInput`))

(fn `StartGame`
  (bind _returnvalue (`GameplayStatics.GetPlayerPawn` 0))
  (bind _hud (`self.HUD`))
  (bind _warmuptext (`/Game/Blueprints/HUD/GameModeHUD.WarmUpText` _hud))
  (bind _announcement (`/Game/Blueprints/HUD/GameModeHUD.Announcement` _hud))
  (bind _asplayer_controller (cast `PlayerController` (`Pawn.GetController` _returnvalue)))
  (`self.EnableInput` _returnvalue _asplayer_controller)
  (set `TextBlock.Text` "" _warmuptext)
  (`Widget.SetIsEnabled` _warmuptext false)
  (set `TextBlock.Text` "" _announcement)
  (`Widget.SetIsEnabled` _announcement false))

(fn `ToTimeFormat`
  (params (Time :type "Float (double-precision)"))
  (returns (FormatTime :type Text))
  (return (`|FormatText` "{minutes}:{seconds}" (`KismetMathLibrary.FFloor64` (/ Time 60.0)) (`KismetTextLibrary.Conv_DoubleToText` (mod Time 60.0) "HalfToEven" false true 2 2 0 0))))

(fn `UpdateGameTimer`
  (params (DeltaTime :type "Float (double-precision)"))
  (returns (Finished :type Boolean))
  (bind _returnvalue (- (`self.GameTime`) DeltaTime))
  (if (<= _returnvalue 0.0)
    (set `TextBlock.Text` "00:00" (`/Game/Blueprints/HUD/GameModeHUD.TimeText` (`self.HUD`)))
    (return true)
    (else
      (bind _output_get (set `self.GameTime` _returnvalue))
      (bind _formattime (`self.ToTimeFormat` _output_get))
      (set `TextBlock.Text` _formattime (`/Game/Blueprints/HUD/GameModeHUD.TimeText` (`self.HUD`)))
      (return false))))

(fn `UpdateWarmup`
  (returns (Finished :type Boolean))
  (bind _returnvalue (`KismetMathLibrary.FCeil64` (- (`self.WarmUpTime`) (`KismetSystemLibrary.GetGameTimeInSeconds`))))
  (if (>= _returnvalue 0)
    (set `TextBlock.Text` (`KismetTextLibrary.Conv_Int64ToText` _returnvalue) (`/Game/Blueprints/HUD/GameModeHUD.WarmUpText` (`self.HUD`)))
    (return false)
    (else
      (return true))))

(fn `UserConstructionScript`)
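; AI controller for BP_Enemy that runs BT_Enemy and turns sight and hearing perception updates into blackboard values.
; Sight updates on the player set chase speed, set or clear TargetActor and record LastKnownLocation; other sighted actors trigger patrol speed.
; Sounds within FlareDetectDistance of the pawn are treated as flares and written to FlareLocation.
; Losing sight of the player still applies chase speed rather than restoring patrol speed.
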(event `self.AIPerception.OnTargetPerceptionUpdated`
  (params (Actor :type "Actor Object Reference") (Stimulus :type "AIStimulus Structure"))
  (`self.HandleHearSense` Actor Stimulus)
  (`self.HandleSightSense` Actor Stimulus))

(event `self.ReceiveBeginPlay`
  (`self.RunBehaviorTree` "/Game/Blueprints/Drone/BT_Enemy.BT_Enemy")
  (set `self.SelfBlackboard` (`AIBlueprintHelperLibrary.GetBlackboard` null))
  (`KismetSystemLibrary.PrintString` "BB Suc"))

(fn `HandleHearSense`
  (params (SightActor :type "Actor Object Reference") (Stimulus :type "AIStimulus Structure"))
  (bind (_age _expirationage _strength _stimuluslocation) (break `AIStimulus` (`local.Stimulus`)))
  (bind _returnvalue (`AIPerceptionSystem.GetSenseClassForStimulus` Stimulus))
  (if (== _returnvalue "/Script/AIModule.AISense_Hearing")
    (if (<= (`KismetMathLibrary.Vector_Distance` (`self.K2_GetActorLocation` (`self.K2_GetPawn`)) _stimuluslocation) (`self.FlareDetectDistance`))
      (`BlackboardComponent.SetValueAsVector` (`self.SelfBlackboard`) "FlareLocation" _stimuluslocation)
      (`KismetSystemLibrary.PrintString` "Hear a sound")
      (return)
      (else
        (`KismetSystemLibrary.PrintString` "This flare is out of distance!")
        (return)))
    (else
      (`KismetSystemLibrary.PrintString` "Hearing cast failed")
      (return))))

(fn `HandleSightSense`
  (params (SightActor :type "Actor Object Reference") (Stimulus :type "AIStimulus Structure"))
  (bind (_age _expirationage _strength _stimuluslocation _receiverlocation _tag _bsuccessfullysensed) (break `AIStimulus` (`local.Stimulus`)))
  (bind _returnvalue (`AIPerceptionSystem.GetSenseClassForStimulus` Stimulus))
  (if (== _returnvalue "/Script/AIModule.AISense_Sight")
    (if (== (`local.SightActor`) (`GameplayStatics.GetPlayerCharacter` 0))
      (`KismetSystemLibrary.PrintString` "SEE Player!")
      (`self.SetSpeed` (`self.ChaseSpeed`))
      (`BlackboardComponent.SetValueAsObject` (`self.SelfBlackboard`) "TargetActor" (select `bool` _bsuccessfullysensed :`true` (`GameplayStatics.GetPlayerCharacter` 0)))
      (if _bsuccessfullysensed
        (`BlackboardComponent.SetValueAsVector` (`self.SelfBlackboard`) "LastKnownLocation" _stimuluslocation)
        (return)
        (else
          (`BlackboardComponent.SetValueAsVector` (`self.SelfBlackboard`) "LastKnownLocation" _stimuluslocation)))
      (else
        (`self.SetSpeed` (`self.PatrolSpeed`))))
    (else
      (return))))

(fn `SetSpeed`
  (params (NewSpeed :type "Float (double-precision)"))
  (bind _asbp_enemy (cast `/Game/Blueprints/Drone/BP_Enemy` (`self.K2_GetPawn`)))
  (set `CharacterMovementComponent.MaxWalkSpeed` NewSpeed (`Character.CharacterMovement` _asbp_enemy))
  (`KismetSystemLibrary.PrintString` (`KismetStringLibrary.Conv_DoubleToString` NewSpeed)))

(fn `UserConstructionScript`)
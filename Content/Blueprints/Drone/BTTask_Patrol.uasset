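; Behavior tree task that sends a BP_Enemy drone along linked PatrolPoint actors, one leg per execution.
; With no current point, it picks a random one from the enemy's PatrolPoints.
; A MoveToPatrolAndWait macro runs AI MoveTo and waits on arrival, then the task advances to the point's NextPoint and finishes successfully.
; A failed move or pawn cast finishes the task as failed.
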(event `self.ReceiveExecuteAI`
  (params (OwnerController :type "AIController Object Reference") (ControlledPawn :type "Pawn Object Reference"))
  (bind _currentpatrolpoint (`self.CurrentPatrolPoint`))
  (bind _asbp_enemy (cast `/Game/Blueprints/Drone/BP_Enemy` ControlledPawn)
    (:`then`
      (`KismetSystemLibrary.PrintString` "Cast Successful to BP Enemy!")
      (`/Engine/EditorBlueprintResources/StandardMacros.IsValid` _currentpatrolpoint
        (:`Is Valid`
          (`self.MoveToPatrolAndWait` _currentpatrolpoint _asbp_enemy
            (:`OnFail`
              (`self.FinishExecute` false))
            (:`OnSuccess`
              (`self.SetNextPatrolPoint`)
              (`self.FinishExecute` true))))
        (:`Is Not Valid`
          (bind _output_get (set `self.CurrentPatrolPoint` (`KismetArrayLibrary.Array_Random` (`/Game/Blueprints/Drone/BP_Enemy.PatrolPoints` _asbp_enemy))))
          (`KismetSystemLibrary.PrintString` (`KismetSystemLibrary.GetDisplayName` _output_get))
          (`self.MoveToPatrolAndWait` _output_get _asbp_enemy
            (:`OnFail`
              (`self.FinishExecute` false))
            (:`OnSuccess`
              (`self.SetNextPatrolPoint`)
              (`self.FinishExecute` true))))))
    (:`CastFailed`
      (`self.FinishExecute` false))))

(fn `SetNextPatrolPoint`
  (bind _aspatrol_point (cast `/Game/Blueprints/Drone/PatrolPoint` (`self.CurrentPatrolPoint`))
    (:`then`
      (set `self.CurrentPatrolPoint` (`/Game/Blueprints/Drone/PatrolPoint.NextPoint` _aspatrol_point))
      (return))
    (:`CastFailed`
      (`KismetSystemLibrary.PrintString` "Somehow current patrol point failed casting!")
      (return))))